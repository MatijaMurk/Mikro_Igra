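; BP_Pickup_AttackRadius is a player pickup that increases the player's attack damage radius.
; It overrides the parent OnPickup, calls it, then scales the player's DamageRadius up by RadiusMultiplier as a percentage.
; The result is clamped between zero and the player's MaxRadius, while the event graph holds only disabled default events.
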(event EventBeginPlay
  (|CallParentFunction) ; This node is disabled and will not be called.\nDrag off pins to build functionality.
)

(event Collision|EventActorBeginOverlap
  (params (OtherActor :type Actor%20Object%20Reference)))

(event EventTick
  (params (DeltaSeconds :type Float%20%28single-precision%29)))

(fn ConstructionScript
  (|CallParentFunction))

(fn OnPickup
  (bind _player (Variables|Default|GetPlayer))
  (|CallParentFunction)
  (Variables|/Game/Player/PlayerCharacter.PlayerCharacter_C|SetDamageRadius _player (Math|Float|Clamp(Float) (* (+ (/ (Variables|Default|GetRadiusMultiplier) 1e+02) 1.0) (Variables|/Game/Player/PlayerCharacter.PlayerCharacter_C|GetDamageRadius _player)) 0.0 (Variables|/Game/Player/PlayerCharacter.PlayerCharacter_C|GetMaxRadius _player))))