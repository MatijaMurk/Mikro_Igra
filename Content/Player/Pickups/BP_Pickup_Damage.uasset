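; BP_Pickup_Damage is a pickup that permanently boosts the player's damage when collected.
; It overrides OnPickup, calling the parent logic and then scaling the player's BaseDamage up by DamageMultiplier, treated as a percentage, so repeated pickups compound.
; All event graph nodes are disabled placeholders, so the rest of its behavior comes from the parent pickup class.
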(event EventBeginPlay
  (|CallParentFunction) ; This node is disabled and will not be called.\nDrag off pins to build functionality.
)

(event Collision|EventActorBeginOverlap
  (params (OtherActor :type Actor%20Object%20Reference)))

(event EventTick
  (params (DeltaSeconds :type Float%20%28single-precision%29)))

(fn ConstructionScript
  (|CallParentFunction))

(fn OnPickup
  (bind _player (Variables|Default|GetPlayer))
  (|CallParentFunction)
  (Variables|/Game/Player/PlayerCharacter.PlayerCharacter_C|SetBaseDamage _player (* (+ (/ (Variables|Default|GetDamageMultiplier) 1e+02) 1.0) (Variables|/Game/Player/PlayerCharacter.PlayerCharacter_C|GetBaseDamage _player))))