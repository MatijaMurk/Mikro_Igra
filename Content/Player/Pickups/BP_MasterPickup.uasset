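; Base pickup actor that announces its pickup type on the player's HUD and destroys itself when its sphere is overlapped.
; BeginPlay caches the player character and the MicroPC controller.
; Any sphere overlap, with no check on the overlapping actor, calls OnPickup before destruction.
; OnPickup adds a new InfoText widget to a HUD vertical box, labeled with the PickupType enum's name.
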(event OnComponentBeginOverlap(Sphere)
  (params (OverlappedComponent :type Primitive%20Component%20Object%20Reference) (OtherActor :type Actor%20Object%20Reference) (OtherComp :type Primitive%20Component%20Object%20Reference) (OtherBodyIndex :type Integer) (bFromSweep :type Boolean) (SweepResult :type Hit%20Result%20Structure%20%28by%20ref%29))
  (CallFunction|OnPickup)
  (Actor|DestroyActor))

(event EventBeginPlay
  (bind _asplayer_character (Utilities|Casting|CastToPlayerCharacter (Game|GetPlayerCharacter 0)))
  (Variables|Default|SetPlayer _asplayer_character)
  (bind _asmicro_pc (Utilities|Casting|CastToMicroPC (Game|GetPlayerController 0)))
  (Variables|Default|SetPlayerPC _asmicro_pc))

(fn ConstructionScript)

(fn OnPickup
  (bind _returnvalue (UserInterface|CreateWidget "/Game/Player/HUD/InfoText.InfoText_C"))
  (bind _output_get (Variables|Default|SetInfoText _returnvalue))
  (Class|VerticalBox|AddChildtoVerticalBox (Variables|/Game/Player/HUD/HUD.HUD_C|GetVerticalBox_89 (Variables|/Game/Player/MicroPC.MicroPC_C|GetHUD (Variables|Default|GetPlayerPC))) _output_get)
  (Rendering|Components|TextRender|SetText (Variables|/Game/Player/HUD/InfoText.InfoText_C|GetItemName (Variables|Default|GetInfoText)) (Utilities|Text|ToText(String) (Utilities|String|EnumtoString (Variables|Default|GetPickupType)))))