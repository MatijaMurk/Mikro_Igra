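; BP_Pickup_FireRate is a player pickup that alters the player's firing speed when collected.
; It overrides OnPickup, calls the parent logic, then treats FireRateMultiplier as a percentage.
; That percentage scales the player's FireRate down and PlayRate up, compounding on the current values with no revert in this Blueprint.
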(event EventBeginPlay)

(event Collision|EventActorBeginOverlap
  (params (OtherActor :type Actor%20Object%20Reference)))

(event EventTick
  (params (DeltaSeconds :type Float%20%28single-precision%29)))

(fn ConstructionScript
  (|CallParentFunction))

(fn OnPickup
  (bind _player (Variables|Default|GetPlayer))
  (bind _fireratemultiplier (Variables|Default|GetFireRateMultiplier))
  (|CallParentFunction)
  (Variables|/Game/Player/PlayerCharacter.PlayerCharacter_C|SetFireRate _player (* (/ (- 1e+02 _fireratemultiplier) 1e+02) (Variables|/Game/Player/PlayerCharacter.PlayerCharacter_C|GetFireRate _player)))
  (Variables|/Game/Player/PlayerCharacter.PlayerCharacter_C|SetPlay%20Rate _player (* (+ (/ _fireratemultiplier 1e+02) 1.0) (Variables|/Game/Player/PlayerCharacter.PlayerCharacter_C|GetPlay%20Rate _player))))