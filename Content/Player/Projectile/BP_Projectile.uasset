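; BP_Projectile is the player's ranged projectile, which deals radial damage with falloff where it hits.
; On BeginPlay it caches the player character, whose stats set the damage and blast radius on impact.
; A hit spawns a Niagara impact effect scaled to that radius, then destroys the actor after a brief delay.
; Without a hit, it plays the same effect at its location and self-destructs after about three seconds.
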(event Collision|EventHit
  (params (MyComp :type Primitive%20Component%20Object%20Reference) (Other :type Actor%20Object%20Reference) (OtherComp :type Primitive%20Component%20Object%20Reference) (bSelfMoved :type Boolean) (HitLocation :type Vector :default "0, 0, 0") (HitNormal :type Vector :default "0, 0, 0") (NormalImpulse :type Vector :default "0, 0, 0") (Hit :type Hit%20Result%20Structure%20%28by%20ref%29))
  (bind _impactpoint (Collision|BreakHitResult Hit))
  (bind _player (Variables|Default|GetPlayer))
  (bind _damageranged (Variables|/Game/Player/PlayerCharacter.PlayerCharacter_C|GetDamageRanged _player))
  (bind _basedamage (Variables|/Game/Player/PlayerCharacter.PlayerCharacter_C|GetBaseDamage _player))
  (bind _damageradius (Variables|/Game/Player/PlayerCharacter.PlayerCharacter_C|GetDamageRadius _player))
  (bind _returnvalue (* _basedamage _damageranged))
  (Class|GameplayStatics|ApplyRadialDamagewithFalloff _returnvalue (* _returnvalue 0.15) _impactpoint (* _damageradius 0.5) _damageradius 0.5 0 0 self (Game|GetPlayerController 0) "ECC_WorldDynamic")
  (bind _returnvalue_2 (Niagara|SpawnSystematLocation "/Game/Player/Particles/FX_Impact_System.FX_Impact_System" _impactpoint))
  (Niagara|SetNiagaraVariable(Float) _returnvalue_2 "Size" (/ _damageradius 4e+01))
  (Utilities|FlowControl|Delay 0.2)
  (Actor|DestroyActor))

(event EventBeginPlay
  (bind _asplayer_character (Utilities|Casting|CastToPlayerCharacter (Game|Player|GetPlayerPawn 0)))
  (Variables|Default|SetPlayer _asplayer_character)
  (Utilities|FlowControl|Delay 2.9)
  (Niagara|SpawnSystematLocation "/Game/Player/Particles/FX_Impact_System.FX_Impact_System" (Transformation|GetActorLocation))
  (Actor|DestroyActor))

(fn ConstructionScript)