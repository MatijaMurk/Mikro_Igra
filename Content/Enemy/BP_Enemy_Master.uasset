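; Base slime enemy Blueprint that attacks the player, takes damage and rewards kills with score and pickups.
; A looping timer sphere-traces forward to start a cooldown-gated attack montage, whose notify re-traces to apply damage, with an attack speed multiplier scaling cooldown and play rate.
; Point and radial hits spawn damage numbers and update the health bar.
; Death drops weighted random loot and bursts Niagara particles using the slime's color-customized dynamic material.
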(event Custom|DamageNumber
  (params (Damage :type Float%20%28single-precision%29) (ImpactPoint :type Vector))
  (bind (_x _y _z) (Math|Vector|BreakVector ImpactPoint))
  (bind _returnvalue (Game|SpawnActorfromClass "/Game/Player/HUD/DMGText.DMGText_C" (Math|Transform|MakeTransform (Math|Vector|MakeVector (Math|Random|RandomFloatinRange (+ _x -25.0) (+ _x 25.0)) _y (+ _z 2e+01)) "0, 0, 0" "1,1,1") "Undefined" 0 0))
  (Default|GetDamage _returnvalue Damage))

(event Custom|Attack
  (bind _baseattackspeed (Variables|Default|GetBaseAttackSpeed))
  (bind _play_rate (Variables|Default|GetPlay%20Rate))
  (bind _attackspeedmultiplier (Variables|Default|GetAttackSpeedMultiplier))
  (bind (_as _pr) (Utilities|AttackSpeedCalc _attackspeedmultiplier _baseattackspeed _attackspeedmultiplier _play_rate))
  (Utilities|Cooldown _as
    (:Completed
      (Animation|Montage|PlayMontage (Variables|Character|GetMesh) "/Game/Enemy/Mesh/Animatin/SlimeEnemy_Anim_Attack_Montage.SlimeEnemy_Anim_Attack_Montage" _pr
        (:OnNotifyBegin
          (CallFunction|CreateAttackSphere))))))

(event EventBeginPlay
  (Variables|Default|SetCurrentHealth (Variables|Default|GetMaxHealth))
  (Utilities|Time|SetTimerbyFunctionName 0 "CheckAttack" 0.1 true))

(event Game|Damage|EventPointDamage
  (params (Damage :type Float%20%28single-precision%29) (DamageType :type Damage%20Type%20Object%20Reference) (HitLocation :type Vector :default "0, 0, 0") (HitNormal :type Vector :default "0, 0, 0") (HitComponent :type Primitive%20Component%20Object%20Reference) (BoneName :type Name :default "None") (ShotFromDirection :type Vector :default "0, 0, 0") (InstigatedBy :type Controller%20Object%20Reference) (DamageCauser :type Actor%20Object%20Reference) (HitInfo :type Hit%20Result%20Structure%20%28by%20ref%29))
  (bind _returnvalue (Math|Float|Truncate Damage))
  (CallFunction|DamageNumber (Math|Conversions|ToFloat(Integer) _returnvalue) (.ImpactPoint (Collision|BreakHitResult HitInfo)))
  (CallFunction|UpdateHealth (Math|Conversions|ToFloat(Integer) _returnvalue)))

(event Game|Damage|EventRadialDamage
  (params (DamageReceived :type Float%20%28single-precision%29) (DamageType :type Damage%20Type%20Object%20Reference) (Origin :type Vector :default "0, 0, 0") (HitInfo :type Hit%20Result%20Structure%20%28by%20ref%29) (InstigatedBy :type Controller%20Object%20Reference) (DamageCauser :type Actor%20Object%20Reference))
  (bind _returnvalue (Math|Float|Truncate DamageReceived))
  (CallFunction|DamageNumber (Math|Conversions|ToFloat(Integer) _returnvalue) (.ImpactPoint (Collision|BreakHitResult HitInfo)))
  (CallFunction|UpdateHealth (Math|Conversions|ToFloat(Integer) _returnvalue)))

(fn ConstructionScript
  (bind _returnvalue (Rendering|Material|CreateDynamicMaterialInstance (Variables|Character|GetMesh) 0 "/Game/Enemy/Material/M_SlimeEnemy.M_SlimeEnemy" "None" :!class /Script/Engine.PrimitiveComponent))
  (Rendering|Material|SetVectorParameterValue _returnvalue "Color1" (Variables|Default|GetColor1) :!class /Script/Engine.MaterialInstanceDynamic)
  (Rendering|Material|SetVectorParameterValue _returnvalue "Color2" (Variables|Default|GetColor2) :!class /Script/Engine.MaterialInstanceDynamic))

(fn UpdateHealth
  (params (DamageTaken :type Float%20%28single-precision%29))
  (bind _output_get (Variables|Default|SetCurrentHealth (- (Variables|Default|GetCurrentHealth) DamageTaken)))
  (bind _ashealth_bar (Utilities|Casting|CastToHealthBar (UserInterface|GetUserWidgetObject (Variables|Default|GetWidget))))
  (Variables|/Game/Enemy/UI/HealthBar.HealthBar_C|SetHealth _ashealth_bar (Math|Float|NormalizetoRange _output_get 0.0 (Variables|Default|GetMaxHealth)))
  (if (not (> _output_get 0.0))
    (CallFunction|DropLoot (Variables|Default|GetNumber%20Of%20Loot) (Variables|Default|GetLootDropWeight))
    (bind _asplayer_character (Utilities|Casting|CastToPlayerCharacter (Game|GetPlayerCharacter 0)))
    (Variables|/Game/Player/PlayerCharacter.PlayerCharacter_C|SetScore _asplayer_character (+ (Variables|/Game/Player/PlayerCharacter.PlayerCharacter_C|GetScore _asplayer_character) (Variables|Default|GetScoreToGive)))
    (bind _returnvalue (Niagara|SpawnSystematLocation "/Game/Enemy/Particles/FX_SlimeBurst_System.FX_SlimeBurst_System" (Transformation|GetActorLocation)))
    (Class|NiagaraComponent|SetVariableMaterial _returnvalue "material2" (Rendering|Material|GetMaterial (Variables|Character|GetMesh) 0))
    (Niagara|SetNiagaraVariable(Float) _returnvalue "Scale" (Variables|Default|GetParticleSize))
    (Actor|DestroyActor)))

(fn CheckAttack
  (bind _returnvalue (Transformation|GetActorLocation))
  (bind _outactors (Actor|GetAllActorsOfClass "/Script/Engine.StaticMeshActor"))
  (bind _returnvalue_2 (Class|KismetSystemLibrary|SphereTraceSinglebyProfile _returnvalue (+ _returnvalue (* (Math|Vector|GetForwardVector (Variables|Character|GetMesh)) (Variables|Default|GetAttackRange))) 5e+01 "Player" false _outactors "None" true "(R=1.000000,G=0.000000,B=0.000000,A=1.000000)" "(R=0.000000,G=1.000000,B=0.000000,A=1.000000)" 1.0))
  (if _returnvalue_2
    (Utilities|FlowControl|DoOnce false
      (:Completed
        (CallFunction|Attack)))))

(fn CreateAttackSphere
  (bind _returnvalue (Transformation|GetActorLocation))
  (bind _outactors (Actor|GetAllActorsOfClass "/Script/Engine.StaticMeshActor"))
  (bind (_outhit _returnvalue_2) (Class|KismetSystemLibrary|SphereTraceSinglebyProfile _returnvalue (+ _returnvalue (* (Math|Vector|GetForwardVector (Variables|Character|GetMesh)) (Variables|Default|GetAttackRange))) 5e+01 "Player" false _outactors "None" true "(R=1.000000,G=0.000000,B=0.000000,A=1.000000)" "(R=0.000000,G=1.000000,B=0.000000,A=1.000000)" 1.0))
  (if _returnvalue_2
    (Game|Damage|ApplyDamage (.HitActor (Collision|BreakHitResult _outhit)) (Variables|Default|GetDamage) 0 0)))

(fn DropLoot
  (params (NumberOfLoot :type Integer) (Weight :type Float%20%28single-precision%29))
  (bind _returnvalue (Transformation|GetActorLocation))
  (bind (_x _y _z) (Math|Vector|BreakVector _returnvalue))
  (for _index (range 1 NumberOfLoot)
    (if (Math|Random|RandomBoolwithWeight Weight)
      (Game|SpawnActorfromClass (Utilities|Select :Index (Math|Random|RandomIntegerinRange 0 3) :Option%200 "/Game/Player/Pickups/BP_Pickup_AttackRadius.BP_Pickup_AttackRadius_C" :Option%201 "/Game/Player/Pickups/BP_Pickup_Damage.BP_Pickup_Damage_C" :Option%202 "/Game/Player/Pickups/BP_Pickup_Health.BP_Pickup_Health_C" :Option%203 "/Game/Player/Pickups/BP_Pickup_FireRate.BP_Pickup_FireRate_C") (Math|Transform|MakeTransform (Math|Vector|MakeVector (+ (Math|Random|RandomFloatinRange -2e+01 2e+01) _x) (+ (Math|Random|RandomFloatinRange -2e+01 2e+01) _y) (+ _z 1e+01)) "0, 0, 0" "1,1,1") "AdjustIfPossibleButDontSpawnIfColliding" 0 0))))